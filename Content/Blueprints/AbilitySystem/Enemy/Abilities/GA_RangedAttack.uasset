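; Enemy gameplay ability for a ranged attack that fires a projectile at the avatar's combat target.
; On activation it turns the avatar toward the target and plays a random tagged attack montage.
; When the montage's gameplay event arrives, it re-reads the target's location and spawns the projectile from the tagged socket.
; An optional pitch override uses the flat-ground ballistic angle from horizontal distance, gravity and speed.
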(event Ability|EventActivateAbility
  (bind _returnvalue (Ability|GetAvatarActorfromActorInfo))
  (bind _returnvalue_2 (Ability|GetAvatarActorfromActorInfo))
  (bind _returnvalue_3 (Transformation|GetActorLocation _returnvalue))
  (bind _returnvalue_4 (Class|EnemyInterface|GetCombatTarget(Message) _returnvalue_2))
  (Class|CombatInterface|UpdateFacingTarget(Message) _returnvalue_2 (Transformation|GetActorLocation _returnvalue_4))
  (bind _returnvalue_5 (Class|CombatInterface|GetAttackMontages(Message) (Ability|GetAvatarActorfromActorInfo)))
  (bind _output_get (Variables|Default|SetTaggedMontage (Class|AuraDamageGameplayAbility|GetRandomTaggedMontagefromArray _returnvalue_5)))
  (|PlayMontageandWaitProxy "None" (.Montage (Utilities|Struct|BreakTaggedMontage _output_get)) 1.0 "None" false 1.0 0.0 false
    (:then
      (Ability|Tasks|WaitGameplayEvent (.MontageTag (Utilities|Struct|BreakTaggedMontage _output_get)) 0 true
        (:EventReceived
          (bind _returnvalue_6 (Class|EnemyInterface|GetCombatTarget(Message) _returnvalue))
          (Variables|Default|SetDistance (Math|Vector|Distance(Vector) (Math|Vector|MakeVector (.x (Transformation|GetActorLocation _returnvalue_6)) (.y (Transformation|GetActorLocation _returnvalue_6)) 0.0) (Math|Vector|MakeVector (.x _returnvalue_3) (.y _returnvalue_3) 0.0)))
          (bind _output_get_2 (Variables|Default|SetPitchAngle (/ (Class|KismetMathLibrary|DegAsin (/ (* (Variables|Default|GetDistance) (Variables|Default|GetGravityAcceleration)) (Math|Float|Square (Variables|Default|GetSpeed)))) 2.0)))
          (Class|AuraProjectileSpell|SpawnProjectile (Transformation|GetActorLocation _returnvalue_6) (.SocketTag (Utilities|Struct|BreakTaggedMontage _output_get)) (Variables|Default|GetShould%20Override%20Pitch) _output_get_2))))))